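; Stats component that tracks health for its owning actor and destroys that actor when health runs out.
; AffectHealth subtracts the given value, clamps the result between zero and MaxHealth, runs IsAlive, prints the health and returns it.
; IsAlive reports whether health is above zero and, as a side effect, destroys the owner when it is not.
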(fn `AffectHealth`
  (params (Value :type "Float (double-precision)"))
  (returns (Output_Get :type "Float (double-precision)"))
  (bind _output_get (set `self.Healh` (`KismetMathLibrary.FClamp` (- (`self.Healh`) Value) 0.0 (`self.MaxHealth`))))
  (`self.IsAlive`)
  (`KismetSystemLibrary.PrintString` (`KismetStringLibrary.Conv_DoubleToString` _output_get))
  (return _output_get))

(fn `IsAlive`
  (returns (IsAlive :type Boolean))
  (if (> (`self.Healh`) 0.0)
    (return true)
    (else
      (`Actor.K2_DestroyActor` (`self.GetOwner`))
      (return false))))